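; Base Paper2D tank character for a multiplayer game, with four-direction movement, turret firing, health and death by explosion.
; Directional inputs set orientation, flipbook and a looping movement timer, cleared on release.
; Authority checks route client orientation, animation and shooting through server events, with multicasts for replication, though host inputs mostly update locally.
; Damage updates the controller's HUD widget and destroys the tank at zero health.
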(event Custom|Update%20Animation
  (params (bIsIdle :type Boolean))
  ;[1 1 1] Update Animation
  (Sprite|SetFlipbook (Variables|Default|GetSprite) (select bIsIdle "/Game/Sprites/Tank/FlipBook_Tank_Idle.FlipBook_Tank_Idle" "/Game/Sprites/Tank/FlipBook_Tank_Move.FlipBook_Tank_Move")))

(event Custom|PlayerOrientation
  (params (MovementState :type E_TankOrientation%20Enum :default "NewEnumerator0"))
  ;[1 1 1] New Movement System
  ;;[1 1 1] PlayerOrientation
  (bind _output_get (Variables|Default|SetMovementState MovementState))
  (Transformation|SetActorRotation (Utilities|Select :Index _output_get :NewEnumerator0 (Transformation|GetActorRotation) :NewEnumerator1 "0, 0, 0" :NewEnumerator2 "0.000000,180.000000,0.000000" :NewEnumerator3 "0.000000,-90.000000,0.000000" :NewEnumerator4 "0.000000,90.000000,0.000000")))

(event Custom|Update%20score
  ;[1 1 1] Update Score
  (Default|UpdateScore (Variables|/Game/Blueprints/GameRelated/BP_TankController.BP_TankController_C|GetDevMapUI_Widget (Variables|Default|GetPlayerController)) (Variables|Default|GetScore)))

(event Custom|Update%20Health
  (bind _playercontroller (Variables|Default|GetPlayerController))
  (bind _devmapui_widget (Variables|/Game/Blueprints/GameRelated/BP_TankController.BP_TankController_C|GetDevMapUI_Widget _playercontroller))
  ;[1 1 1] Update Health Event
  (Development|PrintString (Utilities|String|ToString(Float) (Variables|Default|GetHealth)))
  (Utilities|IsValid _devmapui_widget
    (:Is%20Valid
      (Default|UpdateHealth _devmapui_widget (Variables|Default|GetHealth) (Variables|Default|GetInitialHealth)))))

(event Custom|StopPlayerMovement
  ;[1 1 1] New Movement System
  ;;[1 1 1] StopMovementInput
  (Components|Movement|StopMovementImmediately (Variables|Character|GetCharacterMovement)))

(event Custom|SetCharacterMovement
  ;[1 1 1] New Movement System
  ;;[1 1 1] Move character in appropriate direction
  (Pawn|Input|AddMovementInput (Utilities|Select :Index (Variables|Default|GetMovementState) :NewEnumerator0 "0, 0, 0" :NewEnumerator1 "1.000000,0.000000,0.000000" :NewEnumerator2 "-1.000000,0.000000,0.000000" :NewEnumerator3 "0.000000,-1.000000,0.000000" :NewEnumerator4 "0.000000,1.000000,0.000000") 1.0 false))

(event Input|EnhancedActionEvents|EnhancedInputActionIA_FireTurret
  (params (ActionValue :type Boolean) (ElapsedSeconds :type Float%20%28double-precision%29) (TriggeredSeconds :type Float%20%28double-precision%29) (InputAction :type Input%20Action%20Object%20Reference :default "/Game/Blueprints/Input/IA_FireTurret.IA_FireTurret"))
  ;[1 1 1] Shooting
  (:Started
    (Networking|SwitchHasAuthority
      (:Authority
        (CallFunction|ShootProjectile))
      (:Remote
        (CallFunction|ServerShootProjectile)))))

(event Input|EnhancedActionEvents|EnhancedInputActionIA_MoveUp
  (params (ActionValue :type Boolean) (ElapsedSeconds :type Float%20%28double-precision%29) (TriggeredSeconds :type Float%20%28double-precision%29) (InputAction :type Input%20Action%20Object%20Reference :default "/Game/Blueprints/Input/IA_MoveUp.IA_MoveUp"))
  ;[1 1 1] MoveUp
  (:Started
    (Networking|SwitchHasAuthority
      (:Authority
        (CallFunction|PlayerOrientation "NewEnumerator1")
        (CallFunction|UpdateAnimation false)
        (CallFunction|PlayerMove "NewEnumerator1"))
      (:Remote
        (CallFunction|ServerPlayerOrientation "NewEnumerator1")
        (CallFunction|ServerUpdateAnimation false)
        (CallFunction|PlayerMove "NewEnumerator1"))))
  (:Canceled
    (CallFunction|OnMovementComplete "NewEnumerator1" :!label _label))
  (:Completed
    (goto _label)))

(event Input|EnhancedActionEvents|EnhancedInputActionIA_MoveDown
  (params (ActionValue :type Boolean) (ElapsedSeconds :type Float%20%28double-precision%29) (TriggeredSeconds :type Float%20%28double-precision%29) (InputAction :type Input%20Action%20Object%20Reference :default "/Game/Blueprints/Input/IA_MoveDown.IA_MoveDown"))
  ;[1 1 1] MoveDown
  (:Started
    (Networking|SwitchHasAuthority
      (:Authority
        (CallFunction|PlayerOrientation "NewEnumerator2")
        (CallFunction|UpdateAnimation false)
        (CallFunction|PlayerMove "NewEnumerator2"))
      (:Remote
        (CallFunction|ServerPlayerOrientation "NewEnumerator2")
        (CallFunction|ServerUpdateAnimation false)
        (CallFunction|PlayerMove "NewEnumerator2"))))
  (:Canceled
    (CallFunction|OnMovementComplete "NewEnumerator2" :!label _label))
  (:Completed
    (goto _label)))

(event Input|EnhancedActionEvents|EnhancedInputActionIA_MoveRight
  (params (ActionValue :type Boolean) (ElapsedSeconds :type Float%20%28double-precision%29) (TriggeredSeconds :type Float%20%28double-precision%29) (InputAction :type Input%20Action%20Object%20Reference :default "/Game/Blueprints/Input/IA_MoveRight.IA_MoveRight"))
  ;[1 1 1] MoveRight
  (:Started
    (Networking|SwitchHasAuthority
      (:Authority
        (CallFunction|MulticastOrientation "NewEnumerator4")
        (CallFunction|UpdateAnimation false)
        (CallFunction|PlayerMove "NewEnumerator4"))
      (:Remote
        (CallFunction|ServerPlayerOrientation "NewEnumerator4")
        (CallFunction|ServerUpdateAnimation false)
        (CallFunction|PlayerMove "NewEnumerator4"))))
  (:Canceled
    (CallFunction|OnMovementComplete "NewEnumerator4" :!label _label))
  (:Completed
    (goto _label)))

(event Input|EnhancedActionEvents|EnhancedInputActionIA_MoveLeft
  (params (ActionValue :type Boolean) (ElapsedSeconds :type Float%20%28double-precision%29) (TriggeredSeconds :type Float%20%28double-precision%29) (InputAction :type Input%20Action%20Object%20Reference :default "/Game/Blueprints/Input/IA_MoveLeft.IA_MoveLeft"))
  ;[1 1 1] MoveLeft
  (:Started
    (Networking|SwitchHasAuthority
      (:Authority
        (CallFunction|PlayerOrientation "NewEnumerator3")
        (CallFunction|UpdateAnimation false)
        (CallFunction|PlayerMove "NewEnumerator3"))
      (:Remote
        (CallFunction|ServerPlayerOrientation "NewEnumerator3")
        (CallFunction|ServerUpdateAnimation false)
        (CallFunction|PlayerMove "NewEnumerator3"))))
  (:Canceled
    (CallFunction|OnMovementComplete "NewEnumerator3" :!label _label))
  (:Completed
    (goto _label)))

(event EventBeginPlay
  ;[1 1 1] Event Begin Play
  (Utilities|FlowControl|Delay 0.2)
  (Variables|Default|SetInitialHealth (Variables|Default|GetHealth))
  (bind _asbp_tank_controller (Utilities|Casting|CastToBP_TankController (Pawn|GetController)))
  (Variables|Default|SetPlayerController _asbp_tank_controller))

(event Game|Damage|EventAnyDamage
  (params (Damage :type Float%20%28single-precision%29) (DamageType :type Damage%20Type%20Object%20Reference) (InstigatedBy :type Controller%20Object%20Reference) (DamageCauser :type Actor%20Object%20Reference))
  ;[1 1 1] Recieve Damage
  (Variables|Default|SetHealth (- (Variables|Default|GetHealth) Damage))
  (Utilities|FlowControl|Delay 0.1)
  (CallFunction|UpdateHealth)
  (if (<= (Variables|Default|GetHealth) 0.0)
    (Sprite|SetFlipbook (Variables|Default|GetSprite) "/Game/Sprites/Explosion/FB_Explosion.FB_Explosion")
    (Utilities|FlowControl|Delay 0.36)
    (Actor|DestroyActor)))

(event Custom|Server_UpdateAnimation
  (params (bIsIdle :type Boolean))
  ;[1 1 1] Animation Update
  (CallFunction|ReplicateUpdateAnimation bIsIdle))

(event Custom|Server_PlayerOrientation
  (params (MovementState :type E_TankOrientation%20Enum :default "NewEnumerator0"))
  ;[1 1 1] Serever SetOrientation
  (CallFunction|MulticastOrientation MovementState))

(event Custom|Multicast_Orientation
  (params (NewParam :type E_TankOrientation%20Enum :default "NewEnumerator0"))
  ;[1 1 1] Serever SetOrientation
  (CallFunction|PlayerOrientation NewParam))

(event Custom|Server_StopCharacterMovement
  ;[1 1 1] Stop Movement
  (CallFunction|RaplicateStopMovement))

(event Custom|Raplicate_StopMovement
  ;[1 1 1] Stop Movement
  (CallFunction|StopPlayerMovement))

(event Custom|Server%20Shoot%20Projectile
  ;[1 1 1] Server Shooting
  (CallFunction|ShootProjectile))

(event Custom|Replicate_UpdateAnimation
  (params (bIsIdle :type Boolean))
  ;[1 1 1] Animation Update
  (CallFunction|UpdateAnimation bIsIdle))

(fn ConstructionScript)

(fn ShootProjectile
  (bind _returnvalue (Game|SpawnActorfromClass "/Game/Blueprints/Character/BP_TankProjectile.BP_TankProjectile_C" (Transformation|GetWorldTransform (Variables|Default|GetProjectileSpawn)) "Undefined" "MultiplyWithRoot" 0 2.0 0))
  (Actor|SetOwner _returnvalue self)
  (Variables|/Game/Blueprints/Character/BP_TankProjectile.BP_TankProjectile_C|SetAs%20BP%20Base%20Tank%20Paper%20Character _returnvalue self))

(fn OnMovementComplete
  (params (MovementInput :type E_TankOrientation%20Enum :default "NewEnumerator0"))
  ;[1 1 1] Clear Timer and stop movement
  (if (Utilities|Enum|Equal(Enum) MovementInput (Variables|Default|GetMovementState))
    (Variables|Default|SetMovementState "NewEnumerator0")
    (Utilities|Time|ClearandInvalidateTimerbyHandle (Variables|Default|GetmovementTimerHandle))
    (Networking|SwitchHasAuthority
      (:Authority
        (CallFunction|UpdateAnimation true)
        (Utilities|Time|SetTimerbyEvent (EventDispatchers|CreateEvent :!event Custom|StopPlayerMovement) 0.001))
      (:Remote
        (CallFunction|ServerUpdateAnimation true)
        (Utilities|Time|SetTimerbyEvent (EventDispatchers|CreateEvent :!event Custom|Server_StopCharacterMovement) 0.001)))))

(fn PlayerMove
  (params (MovementInput :type E_TankOrientation%20Enum :default "NewEnumerator0"))
  (if (or (!= (Utilities|Enum|Equal(Enum) (Variables|Default|GetMovementState) MovementInput) false) (Utilities|Enum|Equal(Enum) (Variables|Default|GetMovementState) "NewEnumerator0"))
    (Variables|Default|SetMovementState MovementInput)
    (bind _returnvalue (Utilities|Time|SetTimerbyEvent (EventDispatchers|CreateEvent :!event Custom|SetCharacterMovement) 0.01 true))
    (Variables|Default|SetmovementTimerHandle _returnvalue)))