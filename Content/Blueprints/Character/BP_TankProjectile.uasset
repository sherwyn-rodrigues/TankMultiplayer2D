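; Projectile actor for tank Paper characters that damages a tank it overlaps and destroys itself after a set active time.
; On overlap with anything but its owner it hides, applies fixed damage to tanks, then increments and refreshes a stored tank reference's score before destruction.
; Non-tank hits destroy it directly.
; A timer-based delayed collision enable exists, but its call in this graph is disconnected.
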(event OnComponentBeginOverlap(Box)
  (params (OverlappedComponent :type Primitive%20Component%20Object%20Reference) (OtherActor :type Actor%20Object%20Reference) (OtherComp :type Primitive%20Component%20Object%20Reference) (OtherBodyIndex :type Integer) (bFromSweep :type Boolean) (SweepResult :type Hit%20Result%20Structure%20%28by%20ref%29))
  (bind _as_bp_base_tank_paper_character (Variables|Default|GetAs%20BP%20Base%20Tank%20Paper%20Character))
  ;[1 1 1] On Box Collide
  (if (!= OtherActor (Components|GetOwner))
    (Rendering|SetActorHiddenInGame true)
    (bind _asbp_base_tank_paper_character (Utilities|Casting|CastToBP_BaseTankPaperCharacter 0)
      (:then
        (Game|Damage|ApplyDamage _asbp_base_tank_paper_character 1e+01 0 0)
        (Utilities|IsValid _as_bp_base_tank_paper_character
          (:Is%20Valid
            (Math|Float|IncrementFloat (Variables|/Game/Blueprints/Character/BP_BaseTankPaperCharacter.BP_BaseTankPaperCharacter_C|GetScore _as_bp_base_tank_paper_character)
              (:%20%20
                (Utilities|FlowControl|Delay 0.2)
                (Default|UpdateScore _as_bp_base_tank_paper_character)
                (Actor|DestroyActor))))))
      (:CastFailed
        (Actor|DestroyActor)))))

(event Custom|Set%20Collision
  ;[1 1 1] Set Box Collision
  (Collision|SetCollisionEnabled (Variables|Default|GetBox) "QueryOnly")
  (Utilities|Time|ClearandInvalidateTimerbyHandle (stale Custom|Set%20Box%20Collision _returnvalue)))

(event Custom|SelfDestructAfter
  ;[1 1 1 0.5] Self destroy projectile
  (Utilities|Time|SetTimerbyEvent (delegate Custom|DestroyProjectile) (Variables|Default|GetProjectileActivetime)))

(event Custom|DestroyProjectile
  ;[1 1 1 0.5] Self destroy projectile
  (Actor|DestroyActor))

(event Custom|Set%20Box%20Collision
  ;[1 1 1] Set Box Collision
  (bind _returnvalue (Utilities|Time|SetTimerbyEvent (delegate Custom|Set%20Collision) 0.1)))

(event EventBeginPlay
  ;[1 1 1] Event Begin Play
  (CallFunction|SelfDestructAfter))

(fn ConstructionScript)