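; BP_TankGameMode is a tank game mode that sets up joining players with a HUD and a spawn position.
; BeginPlay caches all PlayerStart actors in an array.
; Each PostLogin increments a player counter, asks the BP_TankController to spawn its HUD and waits briefly.
; It then uses the counter to move that player's character to the matching start's location, if valid.
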(event EventBeginPlay
  ;[1 1 1] Begin Play
  (bind _outactors (Actor|GetAllActorsOfClass "/Script/Engine.PlayerStart"))
  (Variables|Default|SetOut%20Actors _outactors))

(event EventPostLogin
  (params (NewPlayer :type Player%20Controller%20Object%20Reference))
  (bind _player (Variables|Default|GetPlayer))
  (bind _out_actors (Variables|Default|GetOut%20Actors))
  (bind _output (Utilities|Array|Get(acopy) _out_actors _player))
  ;[1 1 1] On Post Login
  (Math|Integer|IncrementInt (Variables|Default|GetPlayer)
    (:%20%20
      (bind _asbp_tank_controller (Utilities|Casting|CastToBP_TankController NewPlayer))
      (Default|SpawnHUDEvent _asbp_tank_controller)
      (Utilities|FlowControl|Delay 0.2)
      (Utilities|IsValid _output
        (:Is%20Valid
          (Transformation|SetActorLocationAndRotation (Game|GetPlayerCharacter (Variables|Default|GetPlayer)) (Transformation|GetActorLocation _output)))))))

(fn ConstructionScript)