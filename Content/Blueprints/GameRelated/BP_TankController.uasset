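; BP_TankController is the player controller for a tank game, setting up input and the player's UI.
; On BeginPlay it adds the tank Enhanced Input mapping context and shows the mouse cursor.
; SpawnHUDevent calls SpawningHUD, which, for local controllers only, displays mobile controls and health/score widgets.
; It also creates and stores Game Won and Game Over widgets without adding them to the viewport.
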(event Custom|Spawn%20HUD%20event
  (CallFunction|SpawningHUD))

(event EventBeginPlay
  (Input|AddMappingContext (PlayerController|LocalPlayerSubsystems|GetEnhancedInputLocalPlayerSubsystem self) "/Game/Blueprints/Input/IMC_TankMappingContext.IMC_TankMappingContext" 0 "(bIgnoreAllPressedKeysUntilRelease=True,bForceImmediately=False,bNotifyUserSettings=False)")
  (Variables|Default|SetbShowMouseCursor true))

(fn ConstructionScript)

(fn SpawningHUD
  (if (Pawn|IsLocalPlayerController)
    (bind _returnvalue (UserInterface|CreateWidget "/Game/Blueprints/UI/WBP_MobileControls.WBP_MobileControls_C"))
    (UserInterface|Viewport|AddtoViewport _returnvalue 0)
    (bind _returnvalue_2 (UserInterface|CreateWidget "/Game/Blueprints/UI/WBP_HealthScore.WBP_HealthScore_C"))
    (bind _output_get (Variables|Default|SetDevMapUI_Widget _returnvalue_2))
    (UserInterface|Viewport|AddtoViewport _output_get 0)
    (bind _returnvalue_3 (UserInterface|CreateWidget "/Game/Blueprints/UI/WBP_GameWon.WBP_GameWon_C"))
    (Variables|Default|SetGame%20Won _returnvalue_3)
    (bind _returnvalue_4 (UserInterface|CreateWidget "/Game/Blueprints/UI/WBP_GameOver.WBP_GameOver_C"))
    (Variables|Default|SetGame%20Over _returnvalue_4)))